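; A controllable pawn that is driven through ROS when connected and by standard Unreal movement input otherwise.
; Each Tick checks ROS initialization, then publishes the input axes as a twist message, negating Y and yaw.
; It then teleports to the received ROS pose, scaling position and negating roll and yaw to convert axis conventions.
; Without ROS, axis events apply control-rotation-relative movement, world-up movement and controller yaw.
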(event `self.ReceiveTick`
  (params (DeltaSeconds :type "Float (single-precision)"))
  (bind _returnvalue (`self.IsROSInitialized`))
  (if _returnvalue
    (`ROSTwistPublisher.PublishTwist` (`self.ROSTwistPublisher`) (`KismetMathLibrary.MakeVector` (stale `InputAxis|MoveForward` AxisValue) (* -1 (stale `InputAxis|MoveRight` AxisValue)) (stale `InputAxis|MoveUp` AxisValue)) (* -1 (stale `InputAxis|Turn` AxisValue)))
    ;[1 1 1] ROS Set position and rotation
    (bind _returnvalue_2 (`self.GetROSPosePosition`))
    (bind _returnvalue_3 (`self.GetROSPoseOrientation`))
    (`self.K2_SetActorLocation` (* _returnvalue_2 (`self.ScalePosition`)) false true)
    (`self.K2_SetActorRotation` (`KismetMathLibrary.MakeRotator` (* -1 (.roll (`KismetMathLibrary.Quat_Rotator` _returnvalue_3))) (.pitch (`KismetMathLibrary.Quat_Rotator` _returnvalue_3)) (* -1 (.yaw (`KismetMathLibrary.Quat_Rotator` _returnvalue_3)))) true)))

(event `InputAxis|MoveForward`
  (params (AxisValue :type "Float (single-precision)"))
  (bind (_returnvalue_roll _returnvalue_pitch _returnvalue_yaw) (`KismetMathLibrary.BreakRotator` (`self.GetControlRotation`)))
  ;[1 1 1] Keyboard translation
  (if (not (stale `self.ReceiveTick` _returnvalue))
    (`self.AddMovementInput` (`KismetMathLibrary.GetForwardVector` (`KismetMathLibrary.MakeRotator` _returnvalue_roll _returnvalue_pitch _returnvalue_yaw)) AxisValue)))

(event `InputAxis|MoveRight`
  (params (AxisValue :type "Float (single-precision)"))
  (bind (_returnvalue_roll _returnvalue_pitch _returnvalue_yaw) (`KismetMathLibrary.BreakRotator` (`self.GetControlRotation`)))
  ;[1 1 1] Keyboard translation
  (if (not (stale `self.ReceiveTick` _returnvalue))
    (`self.AddMovementInput` (`KismetMathLibrary.GetRightVector` (`KismetMathLibrary.MakeRotator` _returnvalue_roll _returnvalue_pitch _returnvalue_yaw)) AxisValue)))

(event `InputAxis|MoveUp`
  (params (AxisValue :type "Float (single-precision)"))
  ;[1 1 1] Keyboard translation
  (if (not (stale `self.ReceiveTick` _returnvalue))
    (`self.AddMovementInput` (0.0 0.0 1.0) AxisValue)))

(event `InputAxis|Turn`
  (params (AxisValue :type "Float (single-precision)"))
  ;[1 1 1] Rotation
  (if (not (stale `self.ReceiveTick` _returnvalue))
    (`self.AddControllerYawInput` AxisValue)))

(fn `UserConstructionScript`)